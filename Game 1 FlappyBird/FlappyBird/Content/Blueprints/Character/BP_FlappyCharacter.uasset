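; BP_FlappyCharacter is the player character for a Flappy Bird-style game, holding the score and handling death on collision.
; On begin play it creates the WBP_Overlay widget and adds it to the viewport.
; Any hit on the capsule or sprite reloads StartupMap, ending the run.
; AddToScore increments Score and pushes the new value to the overlay.
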(event `self.ReceiveBeginPlay`
  (bind _returnvalue (`|CreateWidget` "/Game/Blueprints/UI/WBP_Overlay.WBP_Overlay_C"))
  (`UserWidget.AddToViewport` _returnvalue 0)
  (set `self.Overlay` _returnvalue))

(event `self.CapsuleComponent.OnComponentHit`
  (params (HitComponent :type "PrimitiveComponent Object Reference") (OtherActor :type "Actor Object Reference") (OtherComp :type "PrimitiveComponent Object Reference") (NormalImpulse :type "Vector Structure") (Hit :type "HitResult Structure (by ref)"))
  (`GameplayStatics.OpenLevel` "StartupMap" :!label _label))

(event `self.Sprite.OnComponentHit`
  (params (HitComponent :type "PrimitiveComponent Object Reference") (OtherActor :type "Actor Object Reference") (OtherComp :type "PrimitiveComponent Object Reference") (NormalImpulse :type "Vector Structure") (Hit :type "HitResult Structure (by ref)"))
  (goto _label))

(fn `AddToScore`
  (bind _output_get (set `self.Score` (+ (`self.Score`) 1)))
  (`/Game/Blueprints/UI/WBP_Overlay.SetScore` (`self.Overlay`) _output_get))

(fn `UserConstructionScript`)